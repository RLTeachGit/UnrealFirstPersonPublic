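; Pickup object in the door puzzle test that tracks which player holds it and reports its weight.
; Pickup and Dropped events set and clear the holder reference, which IsPickedUp checks for validity, and print debug messages.
; GetWeight returns the static mesh's mass only when the object is unheld and nearly motionless, otherwise zero.
; Destruction just prints a debug message.
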(event `Pickup`
  (params (PlayerRef :type "/Game/FirstPerson/BP/FirstPersonCharacter Object Reference"))
  ;[1 1 1] Picked up
  (set `self.PlayerHoldingUsRef` PlayerRef)
  (`KismetSystemLibrary.PrintString` (`KismetTextLibrary.Conv_TextToString` (`|FormatText` "Picked up by {Player}" (`KismetTextLibrary.Conv_StringToText` (`KismetSystemLibrary.GetDisplayName` (`self.PlayerHoldingUsRef`)))))))

(event `Dropped`
  ;[1 1 1] Dropped, clear player Holding us ref
  (`KismetSystemLibrary.PrintString` (`KismetTextLibrary.Conv_TextToString` (`|FormatText` "Dropped {Me}" (`KismetTextLibrary.Conv_StringToText` (`KismetSystemLibrary.GetDisplayName` (`self.PlayerHoldingUsRef`))))))
  (set `self.PlayerHoldingUsRef` (`self.NullPlayer`)))

(event `self.ReceiveDestroyed`
  ;[1 1 1] When object falls out of the world, kill box
  (`KismetSystemLibrary.PrintString` "Dead"))

(fn `getWeight`
  (returns (Return :type "Float (double-precision)"))
  ;[1 1 1] Is it picked up?
  (bind _result (`self.IsPickedUp`))
  (if _result
    _
    (elif (<= (`KismetMathLibrary.VSizeSquared` (`self.GetVelocity`)) 0.1)
      ;[1 1 1] When dropped and static get weigh
      (return (`PrimitiveComponent.GetMass` (`self.StaticMeshComponent`)))
      (else
        _)))
  ;[1 1 1] If moving or still picked up, dont count weight
  (return 0.0))

(fn `IsPickedUp`
  (returns (Result :type Boolean))
  ;[1 1 1] Is object picked up right now?
  (return (`KismetSystemLibrary.IsValid` (`self.PlayerHoldingUsRef`))))

(fn `UserConstructionScript`)